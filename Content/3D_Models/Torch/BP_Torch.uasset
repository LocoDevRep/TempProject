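; Torch Blueprint that shows its fire effect and raises its fire sound to full volume once the player has picked up a torch.
; BeginPlay casts the player character to BP_StylizedModularCharacter, then to bp_bodyguard2, with the second cast reached only if the first succeeds.
; Tick polls PickedUpTorch on the modular character, or on the bodyguard when that reference is invalid, and has no branch to extinguish the fire.
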(event EventBeginPlay
  (bind _asbp_stylized_modular_character (Utilities|Casting|CastToBP_StylizedModularCharacter (Game|GetPlayerCharacter 0)))
  (Variables|Default|SetChar%20REF _asbp_stylized_modular_character)
  (bind _asbp_bodyguard_2 (Utilities|Casting|CastTobp_bodyguard2 (Game|GetPlayerCharacter 0)))
  (Variables|Default|SetAs%20Bp%20Bodyguard%202 _asbp_bodyguard_2))

(event EventTick
  (params (DeltaSeconds :type Float%20%28single-precision%29))
  (bind _as_bp_bodyguard_2 (Variables|Default|GetAs%20Bp%20Bodyguard%202))
  (bind _char_ref (Variables|Default|GetChar%20REF))
  (Utilities|IsValid _char_ref
    (:Is%20Valid
      (if (Variables|/Game/StylizedModularChar/Blueprints/BP_StylizedModularCharacter.BP_StylizedModularCharacter_C|GetPickedUpTorch _char_ref)
        (Audio|Components|Audio|SetVolumeMultiplier (Variables|Default|GetFire01_Cue1) 1.0 :!class /Script/Engine.AudioComponent :!label _label)
        (Development|SetHiddeninGame (Variables|Default|GetP_Fire) false false)))
    (:Is%20Not%20Valid
      (Utilities|IsValid _as_bp_bodyguard_2
        (:Is%20Valid
          (if (Variables|/Game/StylizedModularChar/Blueprints/bp_bodyguard2.bp_bodyguard2_C|GetPickedUpTorch _as_bp_bodyguard_2)
            (goto _label)))))))

(fn ConstructionScript)
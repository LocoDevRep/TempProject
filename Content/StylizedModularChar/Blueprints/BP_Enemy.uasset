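; BP_Enemy is a basic enemy that endlessly chases the first BP_StylizedModularCharacter found in the level.
; On BeginPlay it caches that character after a short delay, while a movement loop polls until the reference is valid.
; The loop runs AI Move To toward the target and repeats, pausing after success but retrying immediately on failure, with debug prints for both results.
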(event Custom|GetEnemy
  (Utilities|FlowControl|Delay 1.0)
  (bind _outactors (Actor|GetAllActorsOfClass "/Game/StylizedModularChar/Blueprints/BP_StylizedModularCharacter.BP_StylizedModularCharacter_C"))
  (Variables|Default|SetMyEnemy (Utilities|Array|Get(acopy) _outactors)))

(event Custom|BaseMovement
  (Utilities|IsValid (Variables|Default|GetMyEnemy) :!label _label
    (:Is%20Valid
      (AI|AIMoveTo self "0, 0, 0" (Variables|Default|GetMyEnemy) 3e+01 false
        (:OnSuccess
          (Utilities|FlowControl|Delay 1.0)
          (Development|PrintString "Succes" true true "(R=0.023822,G=1.000000,B=0.000000,A=1.000000)")
          (goto _label))
        (:OnFail
          (Development|PrintString "Fail" true true "(R=1.000000,G=0.000000,B=0.013939,A=1.000000)")
          (goto _label))))
    (:Is%20Not%20Valid
      (Utilities|FlowControl|Delay 1.0)
      (goto _label))))

(event EventBeginPlay
  (Utilities|FlowControl|Sequence
    (:then_0
      (CallFunction|GetEnemy))
    (:then_1
      (CallFunction|BaseMovement))))

(fn ConstructionScript)